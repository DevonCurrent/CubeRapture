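; BP_EnemyCube is an AI enemy pawn that roams and consumes BP_City actors, causing a loss when it grows too large.
; A search box finds cities for AI MoveTo, with random patrol for non-city overlaps and searches repeating after each move.
; Touching a city destroys it and uses its population to enlarge the cube and search box.
; Reaching the size limit pauses the game and shows WBP_Lose.
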(event OnComponentBeginOverlap(Cube)
  (params (OverlappedComponent :type Primitive%20Component%20Object%20Reference) (OtherActor :type Actor%20Object%20Reference) (OtherComp :type Primitive%20Component%20Object%20Reference) (OtherBodyIndex :type Integer) (bFromSweep :type Boolean) (SweepResult :type Hit%20Result%20Structure%20%28by%20ref%29))
  (if (Utilities|ClassIsChildOf (Utilities|GetClass OtherActor) "/Game/CubeRapture/Core/Cities/BP_City.BP_City_C")
    (bind _asbp_city (Utilities|Casting|CastToBP_City OtherActor))
    (CallFunction|IncreaseSize (Variables|/Game/CubeRapture/Core/Cities/BP_City.BP_City_C|GetPopulation _asbp_city))
    ;[1 1 1] Needs to be destroyed on next tick
    (Utilities|FlowControl|Delay 0.0001)
    (Actor|DestroyActor _asbp_city)
    (CallFunction|SearchandConsume)))

(event OnComponentBeginOverlap(Box)
  (params (OverlappedComponent :type Primitive%20Component%20Object%20Reference) (OtherActor :type Actor%20Object%20Reference) (OtherComp :type Primitive%20Component%20Object%20Reference) (OtherBodyIndex :type Integer) (bFromSweep :type Boolean) (SweepResult :type Hit%20Result%20Structure%20%28by%20ref%29))
  ;[1 1 1] If enters hitbox, cube goes after city
  (if (Utilities|ClassIsChildOf (Utilities|GetClass OtherActor) "/Game/CubeRapture/Core/Cities/BP_City.BP_City_C")
    (AI|AIMoveTo 0 (Transformation|GetActorLocation OtherActor) 0 5.0 false
      (:OnSuccess
        _)
      (:OnFail
        _))
    (CallFunction|SearchandConsume)))

(event Custom|IncreaseSize
  (params (PopulationConsumed :type Float%20%28single-precision%29))
  (bind _sizeincreaseratio (Variables|Default|GetSizeIncreaseRatio))
  (bind _cube (Variables|Default|GetCube))
  (bind _returnvalue (/ PopulationConsumed _sizeincreaseratio))
  (bind _relativelocation (Variables|/Script/Engine.SceneComponent|GetRelativeLocation _cube))
  (Variables|Default|SetSearchBoxSize (+ (Variables|Default|GetSearchBoxSize) (/ PopulationConsumed 1e+03)))
  (bind _output_get (Variables|Default|Setsize (+ _returnvalue (Variables|Default|Getsize))))
  (Transformation|SetWorldScale3D (Variables|Default|GetCube) (Math|Vector|MakeVector _output_get _output_get _output_get))
  (Transformation|SetRelativeLocation _cube (Math|Vector|MakeVector (.x _relativelocation) (.y _relativelocation) _returnvalue) false false)
  (Transformation|SetRelativeScale3D (Variables|Default|GetBox) (Variables|Default|GetSearchBoxSize))
  (if (>= (Variables|Default|GetSize) 25.0)
    (Game|SetGamePaused true)
    (bind _returnvalue_2 (UserInterface|CreateWidget "/Game/CubeRapture/Core/WBP_Lose.WBP_Lose_C" (Game|GetPlayerController 0)))
    (UserInterface|Viewport|AddtoViewport _returnvalue_2 0)))

(event Custom|Patrol
  (AI|AIMoveTo self (+ (Transformation|GetActorLocation) (Math|Vector|MakeVector (Math|Random|RandomFloatinRange -2e+03 2e+03) (Math|Random|RandomFloatinRange -2e+03 2e+03) 0.0)) 0 5.0 false
    (:OnSuccess
      _)
    (:OnFail
      _))
  (CallFunction|SearchandConsume))

(event Custom|Search%20and%20Consume
  (for _array_element (Collision|GetOverlappingActors (Variables|Default|GetBox) 0 :!class /Script/Engine.PrimitiveComponent)
    (if (Utilities|ClassIsChildOf (Utilities|GetClass _array_element) "/Game/CubeRapture/Core/Cities/BP_City.BP_City_C")
      (AI|AIMoveTo self (Transformation|GetActorLocation _array_element) _array_element 5.0 false
        (:OnSuccess
          _)
        (:OnFail
          _))
      (Utilities|FlowControl|Delay 0.0001)
      (CallFunction|SearchandConsume)
      (else
        (Utilities|FlowControl|Delay 1.0)
        (CallFunction|Patrol)))))

(event EventBeginPlay
  (CallFunction|SearchandConsume))

(fn ConstructionScript)