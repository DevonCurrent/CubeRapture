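; BP_City is a city actor that shows a name and population and grows through ranked city types.
; On BeginPlay, a rank 0 city picks a random name from the CityNames data table.
; PopulateCity adds Growth to the population below rank 4, refreshing the display.
; At MaxPopulation it spawns the next class from the Cities array at its cube's transform, passes on the name and destroys itself.
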(event Custom|PopulateCity
  ;[1 1 1] Grow population of city. If the city grows so big and is not a rank 4 city, then the city will become a new type.
  (if (<= (Variables|Default|GetCityProgressValue) 3)
    (bind _output_get (Variables|Default|SetPopulation (+ (Variables|Default|GetPopulation) (Variables|Default|GetGrowth))))
    (CallFunction|UpdatePopSize)
    (if (>= _output_get (Variables|Default|GetMaxPopulation))
      (bind _returnvalue (Game|SpawnActorfromClass (Utilities|Array|Get(acopy) (Variables|Default|GetCities) (+ (Variables|Default|GetCityProgressValue) 1)) (Transformation|GetWorldTransform (Variables|Default|GetCube)) "Undefined" 0 0))
      (bind _asbp_city (Utilities|Casting|CastToBP_City _returnvalue))
      (bind _output_get_2 (Variables|BP_City_C|SetCityName _asbp_city (Variables|Default|GetCityName)))
      (Rendering|Components|TextRender|SetText (Variables|BP_City_C|GetCityNameDisplay _asbp_city) (Utilities|Text|ToText(String) _output_get_2))
      (Actor|DestroyActor))))

(event EventBeginPlay
  ;[1 1 1] Initialize the city with a unique name
  (if (== (Variables|Default|GetCityProgressValue) 0)
    (bind _outrownames (DataTable|GetDataTableRowNames "/Game/CubeRapture/Core/Cities/CityNames/CityNames.CityNames"))
    (bind _returnvalue (Utilities|GetDataTableRow "/Game/CubeRapture/Core/Cities/CityNames/CityNames.CityNames" (Utilities|Array|Get(acopy) _outrownames (Math|Random|RandomInteger (Utilities|Array|Length _outrownames))))
      (:then
        (Rendering|Components|TextRender|SetText (Variables|Default|GetCityNameDisplay) (Utilities|Text|ToText(String) (Utilities|Struct|BreakS_Cities _returnvalue)))
        (Variables|Default|SetCityName (Utilities|Struct|BreakS_Cities _returnvalue))
        (CallFunction|UpdatePopSize)))
    (else
      (CallFunction|UpdatePopSize))))

(fn ConstructionScript)

(fn UpdatePopSize
  (Rendering|Components|TextRender|SetText (Variables|Default|GetPopulationDisplay) (Utilities|Text|ToText(String) (Utilities|String|Append "Pop: " (Utilities|String|ToString(Float) (Variables|Default|GetPopulation))))))