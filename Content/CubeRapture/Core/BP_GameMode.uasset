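; Game mode for CubeRapture that periodically triggers population of every city once its BeginGame event runs.
; A looping ten-second timer calls PopulateAllCities, which finds all BP_City actors and runs PopulateCity on each.
; Alongside it, a self-repeating one-second Delay loop counts DeltaTime down and resets it to ten on reaching one, as a separate countdown matching the timer's interval.
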(event Custom|PopulateAllCities
  (bind _outactors (Actor|GetAllActorsOfClass "/Game/CubeRapture/Core/Cities/BP_City.BP_City_C"))
  (for _array_element _outactors
    (Default|PopulateCity _array_element)))

(event Custom|BeginGame
  (Utilities|Time|SetTimerbyEvent (delegate Custom|PopulateAllCities) 1e+01 true)
  (Utilities|FlowControl|Delay 1.0 :!label _label)
  (if (!= (Variables|Default|GetDeltaTime) 1.0)
    (Variables|Default|SetDeltaTime (- (Variables|Default|GetDeltaTime) 1.0))
    (goto _label)
    (else
      (Variables|Default|SetDeltaTime 1e+01)
      (goto _label))))

(fn ConstructionScript)